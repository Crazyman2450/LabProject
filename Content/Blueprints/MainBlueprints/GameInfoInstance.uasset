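; Game instance Blueprint that serves as the central UI manager for menus, loading screens, results, and test and theory screens.
; Each show event lazily creates its widget for player 0, caches it and adds it to the viewport, some at set Z-orders.
; CloseTheory picks a theory widget by index, calls its Close and removes it after a short delay.
; A helper function checks whether a given actor overlaps a box collision.
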(event Custom|ShowMainMenu
  ;[1 1 1] Show the main menu
  (Utilities|IsValid (Variables|Default|GetShow%20MainMenu)
    (:Is%20Valid
      _)
    (:Is%20Not%20Valid
      (bind _returnvalue (UserInterface|CreateWidget "/Game/UI/MainMenu/MainMenu_WB.MainMenu_WB_C" (Game|GetPlayerController 0)))
      (Variables|Default|SetShow%20MainMenu _returnvalue)))
  (UserInterface|Viewport|AddtoViewport (Variables|Default|GetShow%20MainMenu) 0))

(event Custom|ShowEndGameLoadingScreen
  (params (Num :type Integer) (Txt :type String))
  ;[1 1 1] End Game Loading Screen
  (Utilities|IsValid (Variables|Widgets|GetEndGameLoadingScreen)
    (:Is%20Valid
      _)
    (:Is%20Not%20Valid
      (bind _returnvalue (UserInterface|CreateWidget "/Game/UI/Transitions/TransitionLoadingScreen_WB.TransitionLoadingScreen_WB_C" (Game|GetPlayerController 0)))
      (Variables|Widgets|SetEndGameLoadingScreen _returnvalue)))
  (Variables|/Game/UI/Transitions/TransitionLoadingScreen_WB.TransitionLoadingScreen_WB_C|SetTxt _returnvalue Txt)
  (Variables|/Game/UI/Transitions/TransitionLoadingScreen_WB.TransitionLoadingScreen_WB_C|SetNum _returnvalue Num)
  (UserInterface|Viewport|AddtoViewport (Variables|Widgets|GetEndGameLoadingScreen) 0))

(event Custom|Theory_01
  (Utilities|IsValid (Variables|Default|GetTheory01)
    (:Is%20Valid
      _)
    (:Is%20Not%20Valid
      (bind _returnvalue (UserInterface|CreateWidget "/Game/UI/MainMenu/Theory/Theory01WB.Theory01WB_C" (Game|GetPlayerController 0)))
      (Variables|Default|SetTheory01 _returnvalue)))
  (UserInterface|Viewport|AddtoViewport (Variables|Default|GetTheory01) 0))

(event Custom|Theory_02
  (Utilities|IsValid (Variables|Default|GetTheory02)
    (:Is%20Valid
      _)
    (:Is%20Not%20Valid
      (bind _returnvalue (UserInterface|CreateWidget "/Game/UI/MainMenu/Theory/Theory02WB.Theory02WB_C" (Game|GetPlayerController 0)))
      (Variables|Default|SetTheory02 _returnvalue)))
  (UserInterface|Viewport|AddtoViewport (Variables|Default|GetTheory02) 0))

(event Custom|CloseTheory
  (params (Num :type Integer))
  (bind _theory01 (Variables|Default|GetTheory01))
  (bind _theory02 (Variables|Default|GetTheory02))
  (if (== Num 0)
    (Utilities|IsValid _theory01
      (:Is%20Valid
        (Default|Close _theory01)
        (Utilities|FlowControl|Delay 0.5)
        (Widget|RemovefromParent _theory01)))
    (elif (== Num 1)
      (Utilities|IsValid _theory02
        (:Is%20Valid
          (Default|Close _theory02)
          (Utilities|FlowControl|Delay 0.5)
          (Widget|RemovefromParent _theory02))))))

(event Custom|RemoveLoadingScreen02
  (Widget|RemovefromParent (Variables|Default|GetLoadingScreen02)))

(event Custom|ShowResults
  ;[1 1 1] Show Results Screen
  (Utilities|IsValid (Variables|Widgets|GetResultsWB)
    (:Is%20Valid
      _)
    (:Is%20Not%20Valid
      (bind _returnvalue (UserInterface|CreateWidget "/Game/UI/Gameplay/Results_WB.Results_WB_C" (Game|GetPlayerController 0)))
      (Variables|Widgets|SetResultsWB _returnvalue)))
  (UserInterface|Viewport|AddtoViewport (Variables|Widgets|GetResultsWB) 0))

(event Custom|ShowPauseMenu
  ;[1 1 1] Show pause menu
  (Utilities|IsValid (Variables|Widgets|GetPauseMenuWB)
    (:Is%20Valid
      _)
    (:Is%20Not%20Valid
      (bind _returnvalue (UserInterface|CreateWidget "/Game/UI/Gameplay/PauseMenu_WB.PauseMenu_WB_C" (Game|GetPlayerController 0)))
      (Variables|Widgets|SetPauseMenuWB _returnvalue)))
  (UserInterface|Viewport|AddtoViewport (Variables|Widgets|GetPauseMenuWB) 0))

(event Custom|ShowLoadingScreen02
  (Utilities|IsValid (Variables|Default|GetLoadingScreen02)
    (:Is%20Valid
      _)
    (:Is%20Not%20Valid
      (bind _returnvalue (UserInterface|CreateWidget "/Game/UI/Transitions/TransitionLoadingScreen02_WB.TransitionLoadingScreen02_WB_C" (Game|GetPlayerController 0)))
      (Variables|Default|SetLoadingScreen02 _returnvalue)))
  (UserInterface|Viewport|AddtoViewport (Variables|Default|GetLoadingScreen02) 1))

(event Custom|ShowGameLoadingScreen
  ;[1 1 1] Show main loading screen
  (Utilities|IsValid (Variables|Widgets|GetShowLoadingScreen)
    (:Is%20Valid
      _)
    (:Is%20Not%20Valid
      (bind _returnvalue (UserInterface|CreateWidget "/Game/UI/Transitions/StartLoadingScreen_WB.StartLoadingScreen_WB_C" (Game|GetPlayerController 0)))
      (Variables|Widgets|SetShowLoadingScreen _returnvalue)))
  (UserInterface|Viewport|AddtoViewport (Variables|Widgets|GetShowLoadingScreen) 50))

(event Custom|Test_01
  (Utilities|IsValid (Variables|Default|GetTest01)
    (:Is%20Valid
      _)
    (:Is%20Not%20Valid
      (bind _returnvalue (UserInterface|CreateWidget "/Game/UI/MainMenu/Tests/Test01WB.Test01WB_C" (Game|GetPlayerController 0)))
      (Variables|Default|SetTest01 _returnvalue)))
  (UserInterface|Viewport|AddtoViewport (Variables|Default|GetTest01) 0))

(event Custom|Test_02
  (Utilities|IsValid (Variables|Default|GetTest02)
    (:Is%20Valid
      _)
    (:Is%20Not%20Valid
      (bind _returnvalue (UserInterface|CreateWidget "/Game/UI/MainMenu/Tests/Test02WB.Test02WB_C" (Game|GetPlayerController 0)))
      (Variables|Default|SetTest02 _returnvalue)))
  (UserInterface|Viewport|AddtoViewport (Variables|Default|GetTest02) 0))

(fn CharacterOverlappingItem
  (params (OverlappingActor :type Object%20Object%20Reference) (BoxCollision :type Primitive%20Component%20Object%20Reference))
  (bind _array_element (Utilities|Array|ForEachLoopwithBreak (Collision|GetOverlappingActors BoxCollision 0 :!class /Script/Engine.PrimitiveComponent) :!label _label)
    (:LoopBody
      (if (== _array_element OverlappingActor)
        (goto _label Break)))
    (:Completed
      (return (== _array_element OverlappingActor)))))