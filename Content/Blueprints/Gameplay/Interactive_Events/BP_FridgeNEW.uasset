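; Interactive fridge whose two doors the player toggles open and shut, with a looked-up popup widget showing the prompt and a button-press flash.
; Overlapping the collision box shows the popup, and Interact checks overlap and a Ready lock before calling ToggleDoors.
; Two timelines swing the doors by yaw with pitch-randomized sounds, while an electrical hum starts at BeginPlay.
; DoorOpen reads inverted (true means shut), and ToggleDoors ignores its Direction input.
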(event OnComponentBeginOverlap(OverlapCollision)
  (params (OverlappedComponent :type Primitive%20Component%20Object%20Reference) (OtherActor :type Actor%20Object%20Reference) (OtherComp :type Primitive%20Component%20Object%20Reference) (OtherBodyIndex :type Integer) (bFromSweep :type Boolean) (SweepResult :type Hit%20Result%20Structure%20%28by%20ref%29))
  (bind _stationpopupref (Variables|Default|GetStationPopupREF))
  (bind _stationpopupref_2 (Variables|Default|GetStationPopupREF))
  (if (== OtherActor (Variables|Default|GetCharacterREF))
    (Variables|/Game/UI/Gameplay/StationPopup_WB.StationPopup_WB_C|SetShowing _stationpopupref_2 true)
    (Variables|/Game/UI/Gameplay/StationPopup_WB.StationPopup_WB_C|SetTitle_Text _stationpopupref_2 "Fridge")
    (Class|Image|SetBrush (Variables|/Game/UI/Gameplay/StationPopup_WB.StationPopup_WB_C|GetIcon_Image _stationpopupref_2) (Utilities|Struct|MakeSlateBrush "(X=128.000000,Y=128.000000)" "(Left=0.000000,Top=0.000000,Right=0.000000,Bottom=0.000000)" "(SpecifiedColor=(R=1.000000,G=1.000000,B=1.000000,A=1.000000),ColorUseRule=UseColor_Specified)" "/Game/UI/UIAssets/Icon_Fridge.Icon_Fridge" "Image" "NoTile" "NoMirror"))
    (Variables|Default|SetInRange? true)
    (if (Variables|Default|GetDoorOpen)
      (Variables|/Game/UI/Gameplay/StationPopup_WB.StationPopup_WB_C|SetInteract_Term _stationpopupref "Open")
      (else
        (Variables|/Game/UI/Gameplay/StationPopup_WB.StationPopup_WB_C|SetInteract_Term _stationpopupref "Close")))))

(event OnComponentEndOverlap(OverlapCollision)
  (params (OverlappedComponent :type Primitive%20Component%20Object%20Reference) (OtherActor :type Actor%20Object%20Reference) (OtherComp :type Primitive%20Component%20Object%20Reference) (OtherBodyIndex :type Integer))
  (if (== OtherActor (Variables|Default|GetCharacterREF))
    (Variables|/Game/UI/Gameplay/StationPopup_WB.StationPopup_WB_C|SetShowing (Variables|Default|GetStationPopupREF) false)
    (Variables|Default|SetInRange? false)))

(event Custom|ToggleDoors
  (params (Direction :type Boolean))
  (bind _returnvalue (Math|Random|RandomFloatinRange 0.7 1.3))
  (bind _popup (Variables|Default|GetPopup))
  (bind _stationpopupref (Variables|Default|GetStationPopupREF))
  (bind _returnvalue_2 (Transformation|GetWorldLocation _popup))
  (if (Variables|Default|GetDoorOpen)
    (Variables|Default|SetDoorOpen false)
    (Variables|/Game/UI/Gameplay/StationPopup_WB.StationPopup_WB_C|SetInteract_Term _stationpopupref "Close")
    (Audio|PlaySoundatLocation "/Game/Audio/EquipmentSounds/FridgeOpen.FridgeOpen" _returnvalue_2 "0, 0, 0" 2.0 _returnvalue 0.0 "/Game/Audio/EquipmentSounds/Fridge_Attentuation.Fridge_Attentuation" 0 0)
    (Utilities|FlowControl|Sequence
      (:then_0
        (bind _doortimeopenright (Timeline|Timeline_0 PlayFromStart)
          (:Update
            (Transformation|SetRelativeRotation (Variables|Default|GetDoorOpenRight) (Math|Rotator|MakeRotator 0.0 0.0 (* _doortimeopenright (Variables|Default|GetDoorAngleRight))) false false))
          (:Finished
            (Variables|Default|SetReady true :!label _label))))
      (:then_1
        (bind _doortimeopenleft (Timeline|Timeline_1 PlayFromStart)
          (:Update
            (Transformation|SetRelativeRotation (Variables|Default|GetDoorOpenLeft) (Math|Rotator|MakeRotator 0.0 0.0 (* _doortimeopenleft (Variables|Default|GetDoorAngleLeft))) false false))
          (:Finished
            (goto _label)))))
    (else
      (Variables|Default|SetDoorOpen true)
      (Variables|/Game/UI/Gameplay/StationPopup_WB.StationPopup_WB_C|SetInteract_Term _stationpopupref "Open")
      (Audio|PlaySoundatLocation "/Game/Audio/EquipmentSounds/FridgeClosed.FridgeClosed" _returnvalue_2 "0, 0, 0" 2.0 _returnvalue 0.0 "/Game/Audio/EquipmentSounds/Fridge_Attentuation.Fridge_Attentuation" 0 0)
      (Utilities|FlowControl|Sequence
        (:then_0
          (Timeline|Timeline_0 ReverseFromEnd))
        (:then_1
          (Timeline|Timeline_1 ReverseFromEnd))))))

(event EventBeginPlay
  (Utilities|FlowControl|Sequence
    (:then_0
      (bind _asbp_character (Utilities|Casting|CastToBP_Character (Game|GetPlayerCharacter 0)))
      (Variables|Default|SetCharacterREF _asbp_character)
      (bind _asstation_popup_wb (Utilities|Casting|CastToStationPopup_WB (UserInterface|GetUserWidgetObject (Variables|Default|GetPopup))))
      (Variables|Default|SetStationPopupREF _asstation_popup_wb)
      (bind _asgame_info_instance (Utilities|Casting|CastToGameInfoInstance (Game|GetGameInstance)))
      (Variables|Default|SetGameInstanceREF _asgame_info_instance))
    (:then_1
      (bind _returnvalue (Audio|SpawnSoundatLocation "/Game/Audio/EquipmentSounds/ElectricalAmbience_Cue.ElectricalAmbience_Cue" (Transformation|GetWorldLocation (Variables|Default|GetFridge_Fridge_Body)) "0, 0, 0" 1.0 2.0 0.0 "/Game/Audio/EquipmentSounds/Fridge_Attentuation.Fridge_Attentuation" 0))
      (Audio|Components|Audio|Play _returnvalue 0.0))))

(event EventInteract
  (params (PlayerInteracted :type Actor%20Object%20Reference))
  (bind _stationpopupref (Variables|Default|GetStationPopupREF))
  (bind _isoverlapping_ (Default|CharacterOverlappingItem (Variables|Default|GetGameInstanceREF) PlayerInteracted (Variables|Default|GetOverlapCollision)))
  (if _isoverlapping_
    (if (Variables|Default|GetInRange?)
      (if (Variables|Default|GetReady)
        (Variables|Default|SetReady false)
        (Variables|/Game/UI/Gameplay/StationPopup_WB.StationPopup_WB_C|SetButtonDown _stationpopupref true)
        (Utilities|FlowControl|Delay 0.1)
        (Variables|/Game/UI/Gameplay/StationPopup_WB.StationPopup_WB_C|SetButtonDown _stationpopupref false)
        (if (Variables|Default|GetDoorOpen)
          (CallFunction|ToggleDoors false)
          (else
            (CallFunction|ToggleDoors true)))))))

(fn ConstructionScript)