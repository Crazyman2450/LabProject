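; BP_InteractControls is a one-shot tutorial trigger that reacts when the player character enters its Sphere.
; BeginPlay caches the BP_Character player reference.
; On overlap, it fades the interact-controls prompt through the character's HUD widget, disables further sphere overlaps, flags OverlappedInteractControls, and updates the objective to the Glass Cabinet and Conical Flask step.
; It also stops the character's Tutorial03 audio if valid.
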(event OnComponentBeginOverlap(Sphere)
  (params (OverlappedComponent :type Primitive%20Component%20Object%20Reference) (OtherActor :type Actor%20Object%20Reference) (OtherComp :type Primitive%20Component%20Object%20Reference) (OtherBodyIndex :type Integer) (bFromSweep :type Boolean) (SweepResult :type Hit%20Result%20Structure%20%28by%20ref%29))
  (bind _characterref (Variables|Default|GetCharacterREF))
  (bind _tutorial_03audio (Variables|/Game/Character/ThirdPersonBP/Blueprints/BP_Character.BP_Character_C|GetTutorial_03Audio _characterref))
  (if (== OtherActor _characterref)
    (Utilities|FlowControl|Sequence
      (:then_0
        (Default|FadeInteractControls (Variables|/Game/Character/ThirdPersonBP/Blueprints/BP_Character.BP_Character_C|GetHUD_WB (Variables|Default|GetCharacterREF)))
        (Variables|/Script/Engine.PrimitiveComponent|SetbGenerateOverlapEvents (Variables|Default|GetSphere) false)
        (Variables|Default|SetOverlappedInteractControls true)
        (Default|UpdateObjective (Variables|/Game/Character/ThirdPersonBP/Blueprints/BP_Character.BP_Character_C|GetHUD_WB (Variables|Default|GetCharacterREF)) "Open the Glass Cabinet and place a Conical Flask athe the Solution Station"))
      (:then_1
        (Utilities|IsValid _tutorial_03audio
          (:Is%20Valid
            (Audio|Components|Audio|Stop _tutorial_03audio)))))))

(event EventBeginPlay
  (bind _asbp_character (Utilities|Casting|CastToBP_Character (Game|GetPlayerCharacter 0)))
  (Variables|Default|SetCharacterREF _asbp_character))

(fn ConstructionScript)