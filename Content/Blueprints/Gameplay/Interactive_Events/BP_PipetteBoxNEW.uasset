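; Interactive pipette box Blueprint that responds to look-at and use events from the player.
; On BeginPlay it flips the lid with a random yaw and caches the game instance and player character.
; Look-at stores the looking character.
; Use, gated by a Ready flag, only prints whether that character holds an item, with no further behavior implemented.
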(event EventBeginPlay
  (Transformation|SetWorldRotation (Variables|Default|GetPipetteBox_Lid) (Math|Rotator|MakeRotator 1.8e+02 0.0 (Math|Random|RandomFloatinRange 5.0 85.0)) false false)
  (bind _asgame_info_instance (Utilities|Casting|CastToGameInfoInstance (Game|GetGameInstance)))
  (Variables|Default|SetGameInfoInstanceREF _asgame_info_instance)
  (bind _asbp_character (Utilities|Casting|CastToBP_Character (Game|GetPlayerCharacter 0)))
  (Variables|Default|SetCharacter%20REF _asbp_character))

(event EventUseItem
  (params (PlayerCharacter :type BP%20Character%20Object%20Reference))
  (if (Variables|Default|GetReady)
    (Variables|/Game/Character/ThirdPersonBP/Blueprints/BP_Character.BP_Character_C|GetCurrentItem PlayerCharacter
      (:then
        (Development|PrintString "item"))
      (:else
        (Development|PrintString "no item")))))

(event EventLookat
  (params (PlayerCharacter :type BP%20Character%20Object%20Reference))
  (Variables|Default|SetPlayer%20Character PlayerCharacter))

(fn ConstructionScript)