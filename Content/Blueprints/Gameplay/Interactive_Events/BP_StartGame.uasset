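; BP_StartGame is a one-shot trigger actor that starts the game's HUD intro and sets the current objective.
; On BeginPlay it caches the player's BP_Character.
; When that character enters its Sphere, it calls FadeStartGame on the HUD widget, passes in its objective name and description, and calls UpdateObjective with "Welcome".
; It then destroys itself.
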(event OnComponentBeginOverlap(Sphere)
  (params (OverlappedComponent :type Primitive%20Component%20Object%20Reference) (OtherActor :type Actor%20Object%20Reference) (OtherComp :type Primitive%20Component%20Object%20Reference) (OtherBodyIndex :type Integer) (bFromSweep :type Boolean) (SweepResult :type Hit%20Result%20Structure%20%28by%20ref%29))
  (bind _characterref (Variables|Default|GetCharacterREF))
  (bind _hud_wb (Variables|/Game/Character/ThirdPersonBP/Blueprints/BP_Character.BP_Character_C|GetHUD_WB _characterref))
  (if (== OtherActor (Variables|Default|GetCharacterREF))
    (Default|FadeStartGame (Variables|/Game/Character/ThirdPersonBP/Blueprints/BP_Character.BP_Character_C|GetHUD_WB (Variables|Default|GetCharacterREF)))
    (Variables|/Game/UI/Objectives/NEWObjectivesHUD_WB.NEWObjectivesHUD_WB_C|SetObjectiveName _hud_wb (Variables|Default|GetCurrentObjectiveName))
    (Variables|/Game/UI/Objectives/NEWObjectivesHUD_WB.NEWObjectivesHUD_WB_C|SetObjectiveDescription _hud_wb (Variables|Default|GetCurrentObjectiveDescription))
    (Default|UpdateObjective (Variables|/Game/Character/ThirdPersonBP/Blueprints/BP_Character.BP_Character_C|GetHUD_WB (Variables|Default|GetCharacterREF)) "Welcome")
    (Actor|DestroyActor)))

(event EventBeginPlay
  (bind _asbp_character (Utilities|Casting|CastToBP_Character (Game|GetPlayerCharacter 0)))
  (Variables|Default|SetCharacterREF _asbp_character))

(fn ConstructionScript)