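; Solution-prep station where the player places an empty conical flask, then adds solutions to make an Intracellular Solution.
; BeginPlay spawns solution items in threes at shuffled SpawnPos actors; used items respawn at their start transforms.
; Each pour updates the board and runs timeline-driven pipette animation and dynamic-material blending of flask fill and colour.
; Eight pours spawn the final item, while Tutorial_Map instead enables the microscope step after three.
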(event OnComponentBeginOverlap(Sphere)
  (params (OverlappedComponent :type Primitive%20Component%20Object%20Reference) (OtherActor :type Actor%20Object%20Reference) (OtherComp :type Primitive%20Component%20Object%20Reference) (OtherBodyIndex :type Integer) (bFromSweep :type Boolean) (SweepResult :type Hit%20Result%20Structure%20%28by%20ref%29))
  (bind _stationpopupref (Variables|Default|GetStationPopupREF))
  ;[1 1 1] Show the description widget
  (if (== OtherActor (Variables|Default|GetCharacterREF))
    (Variables|/Game/UI/Gameplay/StationPopup_WB.StationPopup_WB_C|SetShowing _stationpopupref true)
    (Variables|/Game/UI/Gameplay/StationPopup_WB.StationPopup_WB_C|SetTitle_Text _stationpopupref "Solution Prep")
    (Variables|/Game/UI/Gameplay/StationPopup_WB.StationPopup_WB_C|SetInteractable _stationpopupref false)
    (Class|Image|SetBrush (Variables|/Game/UI/Gameplay/StationPopup_WB.StationPopup_WB_C|GetIcon_Image _stationpopupref) (Utilities|Struct|MakeSlateBrush "(X=128.000000,Y=128.000000)" "(Left=0.000000,Top=0.000000,Right=0.000000,Bottom=0.000000)" "(SpecifiedColor=(R=1.000000,G=1.000000,B=1.000000,A=1.000000),ColorUseRule=UseColor_Specified)" "/Game/UI/UIAssets/Icon_Solution.Icon_Solution" "Image" "NoTile" "NoMirror"))))

(event OnComponentEndOverlap(Sphere)
  (params (OverlappedComponent :type Primitive%20Component%20Object%20Reference) (OtherActor :type Actor%20Object%20Reference) (OtherComp :type Primitive%20Component%20Object%20Reference) (OtherBodyIndex :type Integer))
  ;[1 1 1] Show the description widget
  (if (== OtherActor (Variables|Default|GetCharacterREF))
    (Variables|/Game/UI/Gameplay/StationPopup_WB.StationPopup_WB_C|SetShowing (Variables|Default|GetStationPopupREF) false)))

(event Custom|PourSolution
  (params (Index :type Integer))
  (bind _pipette_pipetteplunger (Variables|Default|GetPipette_PipettePlunger))
  (bind _dynamicmaterial2 (Variables|Default|GetDynamicMaterial2))
  (bind _pipette_pipettebody (Variables|Default|GetPipette_PipetteBody))
  (bind _beaker (Variables|Default|GetBeaker))
  (bind _pipette_pipettebody_2 (Variables|Default|GetPipette_PipetteBody))
  (bind _pipette_pipetteplunger_2 (Variables|Default|GetPipette_PipettePlunger))
  (bind _beaker_2 (Variables|Default|GetBeaker))
  (bind _beaker_full (Variables|Default|GetBeaker_Full))
  (bind _solutioninfo (Variables|Default|GetSolutionInfo))
  (bind _dynamicmaterial1 (Variables|Default|GetDynamicMaterial1))
  (bind _dynamicmaterial2_2 (Variables|Default|GetDynamicMaterial2))
  (bind _returnvalue (Transformation|GetWorldLocation _beaker_full))
  (bind _returnvalue_2 (Transformation|GetWorldTransform _beaker))
  (bind _returnvalue_3 (Transformation|GetWorldTransform _pipette_pipettebody_2))
  (bind _returnvalue_4 (Transformation|GetWorldTransform _pipette_pipetteplunger_2))
  (bind _returnvalue_5 (Transformation|GetWorldTransform _pipette_pipettebody))
  (bind _returnvalue_6 (Transformation|GetWorldTransform _pipette_pipetteplunger))
  (bind _output (Utilities|Array|Get(acopy) (.solutioncolours _solutioninfo) Index))
  ;[1 1 1] Pour Solution
  (Utilities|Array|Add (Variables|Default|GetPlayersSolution) (Utilities|Array|Get(acopy) (.solutionnames _solutioninfo) Index))
  (if (== (Utilities|Array|LastIndex (Variables|Default|GetPlayersSolution)) 7)
    (Default|UpdateMessage (Variables|/Game/Character/ThirdPersonBP/Blueprints/BP_Character.BP_Character_C|GetPickupHUD (Variables|Default|GetPlayer)) "Solution Complete!")
    (else
      (Default|UpdateMessage (Variables|/Game/Character/ThirdPersonBP/Blueprints/BP_Character.BP_Character_C|GetPickupHUD (Variables|Default|GetPlayer)) "Find a Solution to Add")))
  (Default|CallUpdateBoard)
  (Rendering|Material|SetScalarParameterValue _dynamicmaterial2 "Liquid_FillHeight" (Utilities|Array|Get(acopy) (.solutionheights _solutioninfo) Index) :!class /Script/Engine.MaterialInstanceDynamic)
  (Rendering|Material|SetVectorParameterValue _dynamicmaterial2 "Foam_Color" _output :!class /Script/Engine.MaterialInstanceDynamic)
  (Rendering|Material|SetVectorParameterValue _dynamicmaterial2 "Liquid_Color" _output :!class /Script/Engine.MaterialInstanceDynamic)
  (Rendering|SetVisibility (Variables|Default|GetBeaker_Full) true false)
  (bind _returnvalue_7 (Rendering|Material|GetVectorParameterValue (Variables|Default|GetDynamicMaterial1) "Liquid_Color" :!class /Script/Engine.MaterialInstanceDynamic))
  (Transformation|SetWorldLocation (Variables|Default|GetPipette_PipetteBody) (Math|Vector|MakeVector (.x _returnvalue) (.y _returnvalue) (.z _returnvalue)) false false)
  (CallFunction|TogglePipette true)
  (Utilities|FlowControl|Delay 0.5)
  (CallFunction|Anim 1 (Math|Transform|MakeTransform (Math|Vector|MakeVector (.x (.location _returnvalue_4)) (.y (.location _returnvalue_4)) (+ (.z (.location _returnvalue_4)) 4.0)) "0, 0, 0" (.scale _returnvalue_4)))
  (bind _returnvalue_8 (Rendering|Material|GetScalarParameterValue _dynamicmaterial2_2 "Liquid_FillHeight" :!class /Script/Engine.MaterialInstanceDynamic))
  (bind _distance (Timeline|Timeline_2 PlayFromStart)
    (:Update
      (Rendering|Material|SetScalarParameterValue _dynamicmaterial2_2 "Liquid_FillHeight" (Math|Float|Lerp _returnvalue_8 -0.5 _distance) :!class /Script/Engine.MaterialInstanceDynamic))
    (:Finished
      (CallFunction|Anim 0 (Math|Transform|MakeTransform (Math|Vector|MakeVector (.x (.location _returnvalue_5)) (.y (.location _returnvalue_5)) (+ (.z (.location _returnvalue_5)) 5e+01)) (Transformation|GetWorldRotation (Variables|Default|GetPipette_PipetteBody)) (.scale _returnvalue_5)))
      (Utilities|FlowControl|Delay 0.5)
      (CallFunction|Anim 0 (Math|Transform|MakeTransform (Math|Vector|MakeVector (.x (.location _returnvalue_2)) (.y (.location _returnvalue_2)) (+ (.z (.location _returnvalue_2)) 65.0)) (Transformation|GetWorldRotation (Variables|Default|GetPipette_PipetteBody))))
      (Utilities|FlowControl|Delay 0.5)
      (CallFunction|Anim 0 (Math|Transform|MakeTransform (Math|Vector|MakeVector (.x (.location _returnvalue_3)) (.y (.location _returnvalue_3)) (- (.z (.location _returnvalue_3)) 3e+01)) (Transformation|GetWorldRotation (Variables|Default|GetPipette_PipetteBody))))
      (Utilities|FlowControl|Delay 0.5)
      (CallFunction|Anim 1 (Math|Transform|MakeTransform (Math|Vector|MakeVector (.x (.location _returnvalue_6)) (.y (.location _returnvalue_6)) (- (.z (.location _returnvalue_6)) 4.0)) "0, 0, 0" (.scale _returnvalue_6)))
      (Audio|PlaySoundatLocation "/Game/Audio/Water_Pour_3.Water_Pour_3" (Transformation|GetWorldLocation (Variables|Default|GetPipette_PipetteBody)) "0, 0, 0" 1.0 1.0 0.0 0 0 0)
      (bind _distance_2 (Timeline|Timeline_0 PlayFromStart)
        (:Update
          (Rendering|Material|SetScalarParameterValue _dynamicmaterial1 "Liquid_FillHeight" (Math|Float|Lerp (Variables|Default|GetSolutionFill) (+ (Variables|Default|GetSolutionFill) 0.1) _distance_2) :!class /Script/Engine.MaterialInstanceDynamic)
          (Rendering|Material|SetVectorParameterValue _dynamicmaterial1 "Foam_Color" (Math|Color|Lerp(LinearColor) _returnvalue_7 _output _distance_2) :!class /Script/Engine.MaterialInstanceDynamic)
          (Rendering|Material|SetVectorParameterValue _dynamicmaterial1 "Liquid_Color" (Math|Color|Lerp(LinearColor) _returnvalue_7 _output _distance_2) :!class /Script/Engine.MaterialInstanceDynamic))
        (:Finished
          (Variables|Default|SetSolutionFill (+ (Variables|Default|GetSolutionFill) 0.1))
          (CallFunction|TogglePipette false)
          (Rendering|SetVisibility (Variables|Default|GetBeaker_Full) false false)
          (bind _returnvalue_9 (Game|GetCurrentLevelName true))
          ;[1 1 1] Spawn Final Solution
          (if (Utilities|Enum|Equal(Enum) _returnvalue_9 "Tutorial_Map")
            (if (== (Utilities|Array|LastIndex (Variables|Default|GetPlayersSolution)) 2)
              (bind _returnvalue_10 (Audio|SpawnSound2D "/Game/Audio/Tutorial_Voiceover/Tutorial_07.Tutorial_07" 1.0 1.0 0.0 0))
              (Variables|Default|SetTutorial_07Audio _returnvalue_10)
              (bind _outactors (Actor|GetAllActorsOfClass "/Game/Blueprints/Gameplay/Interactive_Events/BP_MicroscopeControls.BP_MicroscopeControls_C"))
              (for _array_element _outactors
                (Variables|/Script/Engine.PrimitiveComponent|SetbGenerateOverlapEvents (Variables|/Game/Blueprints/Gameplay/Interactive_Events/BP_MicroscopeControls.BP_MicroscopeControls_C|GetSphere _array_element) true)
                (Default|UpdateObjective (Variables|/Game/Character/ThirdPersonBP/Blueprints/BP_Character.BP_Character_C|GetHUD_WB (Variables|Default|GetCharacterREF)) "Go to the Main Room and learn the Infrared Microscope Controls"))
              (else
                (CallFunction|SetReady)))
            (elif (== (Utilities|Array|LastIndex (Variables|Default|GetPlayersSolution)) 7)
              (Rendering|SetVisibility _beaker_2 false false)
              (Collision|SetCollisionEnabled _beaker_2 "NoCollision")
              (bind _returnvalue_11 (Rendering|Material|GetVectorParameterValue (Variables|Default|GetDynamicMaterial1) "Liquid_Color" :!class /Script/Engine.MaterialInstanceDynamic))
              (bind _returnvalue_12 (Game|SpawnActorfromClass "/Game/Blueprints/Gameplay/Pickup_Items/Solution_Main.Solution_Main_C" (Transformation|GetWorldTransform (Variables|Default|GetFinalSpawn)) "AdjustIfPossibleButAlwaysSpawn" 0 "Intracellular Solution" "Intracellular Solution is a fluid designed to mimic the ionic content of a cell. It is one of the most important solutions in electrophysiology recordings, yet one of the most difficult to get right." (Variables|Default|GetSolutionFill) _returnvalue_11 0))
              (Variables|/Game/Blueprints/Gameplay/Pickup_Items/ItemParent.ItemParent_C|SetItemDescription _returnvalue_12 "Description of Final Solution")
              (else
                (CallFunction|SetReady)))))))))

(event Custom|SetReady
  ;[1 1 1] Set Ready
  (Utilities|FlowControl|Delay (Variables|Default|GetDebounceTime))
  (Variables|Default|SetReady true))

(event Custom|Holding%20Nothing
  (bind _player (Variables|Default|GetPlayer))
  (bind _pickuphud (Variables|/Game/Character/ThirdPersonBP/Blueprints/BP_Character.BP_Character_C|GetPickupHUD _player))
  ;[1 1 1] Holding Nothing
  (if (Variables|Default|GetFlaskPlaced)
    (Default|UpdateMessage _pickuphud "Find a Solution to Add")
    (else
      (Default|UpdateMessage _pickuphud "Find a Empty Conical Flask"))))

(event Custom|PlaceFlask
  (params (CurrentItem :type Item%20Parent%20Object%20Reference))
  ;[1 1 1] Place Conical Flask
  (Variables|Default|SetFlaskPlaced true)
  (Default|UpdateMessage (Variables|/Game/Character/ThirdPersonBP/Blueprints/BP_Character.BP_Character_C|GetPickupHUD (Variables|Default|GetPlayer)) "Find a Solution to Add")
  (Rendering|SetVisibility (Variables|Default|GetSM_Lab_Cork) true false)
  (Audio|PlaySoundatLocation "/Game/Audio/EquipmentSounds/BottleCorkOpening.BottleCorkOpening" (Variables|/Script/Engine.SceneComponent|GetRelativeLocation (Variables|Default|GetSM_Lab_Bunsen_Stand)) "0, 0, 0" 0.5 0.75 0.05 0 0 0)
  (Audio|PlaySound2D "/Game/Audio/Tutorial_Voiceover/Tutorial_06.Tutorial_06" 1.0 1.0 0.0 0 0)
  (Actor|DestroyActor CurrentItem)
  (CallFunction|SetReady))

(event Custom|SpawnSolutions
  (bind _solutioninfo (Variables|Default|GetSolutionInfo))
  (bind _solutioninfo_2 (Variables|Default|GetSolutionInfo))
  (bind _solutioninfo_3 (Variables|Default|GetSolutionInfo))
  ;[1 1 1] Spawn Solutions
  (bind _outactors (Actor|GetAllActorsOfClass "/Game/Blueprints/Gameplay/Pickup_Items/SpawnPos.SpawnPos_C"))
  (Utilities|Array|Shuffle _outactors)
  (for _array_element _outactors
    (Game|SpawnActorfromClass "/Game/Blueprints/Gameplay/Pickup_Items/Solution_Main.Solution_Main_C" (Transformation|GetActorTransform _array_element) "Undefined" 0 (Utilities|Text|ToText(String) (Utilities|Array|Get(acopy) (.solutionnames _solutioninfo_2) (Variables|Default|GetSolutionLoadNum))) "-" (Utilities|Array|Get(acopy) (.solutionheights _solutioninfo_2) (Variables|Default|GetSolutionLoadNum)) (Utilities|Array|Get(acopy) (.solutioncolours _solutioninfo_2) (Variables|Default|GetSolutionLoadNum)) 0)
    (Game|SpawnActorfromClass "/Game/Blueprints/Gameplay/Pickup_Items/Solution_Main.Solution_Main_C" (Math|Transform|MakeTransform (Math|Vector|MakeVector (.x (.location (Transformation|GetActorTransform _array_element))) (+ (.y (.location (Transformation|GetActorTransform _array_element))) 4e+01) (.z (.location (Transformation|GetActorTransform _array_element)))) (.rotation (Transformation|GetActorTransform _array_element)) (.scale (Transformation|GetActorTransform _array_element))) "Undefined" 0 (Utilities|Text|ToText(String) (Utilities|Array|Get(acopy) (.solutionnames _solutioninfo_3) (- (Variables|Default|GetSolutionLoadNum) 1))) "-" (Utilities|Array|Get(acopy) (.solutionheights _solutioninfo_3) (- (Variables|Default|GetSolutionLoadNum) 1)) (Utilities|Array|Get(acopy) (.solutioncolours _solutioninfo_3) (- (Variables|Default|GetSolutionLoadNum) 1)) 0)
    (Game|SpawnActorfromClass "/Game/Blueprints/Gameplay/Pickup_Items/Solution_Main.Solution_Main_C" (Math|Transform|MakeTransform (Math|Vector|MakeVector (.x (.location (Transformation|GetActorTransform _array_element))) (- (.y (.location (Transformation|GetActorTransform _array_element))) 4e+01) (.z (.location (Transformation|GetActorTransform _array_element)))) (.rotation (Transformation|GetActorTransform _array_element)) (.scale (Transformation|GetActorTransform _array_element))) "Undefined" 0 (Utilities|Text|ToText(String) (Utilities|Array|Get(acopy) (.solutionnames _solutioninfo) (+ (Variables|Default|GetSolutionLoadNum) 1))) "-" (Utilities|Array|Get(acopy) (.solutionheights _solutioninfo) (+ (Variables|Default|GetSolutionLoadNum) 1)) (Utilities|Array|Get(acopy) (.solutioncolours _solutioninfo) (+ (Variables|Default|GetSolutionLoadNum) 1)) 0)
    (Variables|Default|SetSolutionLoadNum (+ (Variables|Default|GetSolutionLoadNum) 3))))

(event Custom|Anim
  (params (ID :type Integer) (Transform :type Transform))
  (bind _pipette_pipetteplunger (Variables|Default|GetPipette_PipettePlunger))
  (bind _pipette_pipettebody (Variables|Default|GetPipette_PipetteBody))
  (bind _array (Utilities|Array|MakeArray _pipette_pipettebody _pipette_pipetteplunger))
  (bind _output (Utilities|Array|Get(acopy) _array ID))
  ;[1 1 1] Animate Pipette
  (bind _animations (Timeline|Timeline_1 PlayFromStart)
    (:Update
      (Transformation|SetWorldTransform _output (Math|Transform|Lerp(Transform) (Transformation|GetWorldTransform _output) Transform _animations) false false))))

(event Custom|TogglePipette
  (params (Visible :type Boolean))
  ;[1 1 1] Toggle Pipette Visibility
  (Rendering|SetVisibility (Variables|Default|GetPipette_PipetteBody) Visible false))

(event EventUseItem
  (params (PlayerCharacter :type BP%20Character%20Object%20Reference))
  ;[1 1 1] Use Solution
  (if (Variables|Default|GetReady)
    (Variables|Default|SetReady false)
    (if (Variables|Default|GetFlaskPlaced)
      (if (not (== (Utilities|Array|LastIndex (Variables|Default|GetPlayersSolution)) 7))
        (bind _currentitem (Variables|/Game/Character/ThirdPersonBP/Blueprints/BP_Character.BP_Character_C|GetCurrentItem PlayerCharacter)
          (:then
            (Variables|Default|SetFoundSolution false)
            (bind (_array_element _array_index) (Utilities|Array|ForEachLoopwithBreak (Variables|Default|GetNEW_Solution_List) :!label _label)
              (:LoopBody
                (if (Utilities|Enum|Equal(Enum) _array_element (Utilities|String|ToString(Text) (Variables|/Game/Blueprints/Gameplay/Pickup_Items/ItemParent.ItemParent_C|GetItemName _currentitem)))
                  (Utilities|FlowControl|Sequence
                    (:then_0
                      (goto _label Break))
                    (:then_1
                      (Variables|Default|SetFoundSolution true)
                      (CallFunction|PourSolution _array_index)
                      (Utilities|FlowControl|Delay 0.1)
                      ;[1 1 1] Respawn Item After Use
                      (bind _outactors (Actor|GetAllActorsOfClass "/Game/Blueprints/Gameplay/Pickup_Items/ItemParent.ItemParent_C"))
                      (bind _array_element_2 (Utilities|Array|ForEachLoopwithBreak _outactors :!label _label_2)
                        (:LoopBody
                          (if (== _array_element_2 (Variables|/Game/Character/ThirdPersonBP/Blueprints/BP_Character.BP_Character_C|GetCurrentItem (Variables|Default|GetPlayer)))
                            (Game|SpawnActorfromClass "/Game/Blueprints/Gameplay/Pickup_Items/Solution_Main.Solution_Main_C" (Variables|/Game/Blueprints/Gameplay/Pickup_Items/ItemParent.ItemParent_C|GetStart_Transform _array_element_2) "Undefined" 0 (Variables|/Game/Blueprints/Gameplay/Pickup_Items/ItemParent.ItemParent_C|GetItemName _array_element_2) "-" (Variables|/Game/Blueprints/Gameplay/Pickup_Items/ItemParent.ItemParent_C|GetFillHeight _array_element_2) (Variables|/Game/Blueprints/Gameplay/Pickup_Items/ItemParent.ItemParent_C|GetFillColour _array_element_2) 0)
                            (Actor|DestroyActor _array_element_2)
                            (goto _label_2 Break))))))))
              (:Completed
                (if (not (Variables|Default|GetFoundSolution))
                  (CallFunction|SetReady)))))
          (:else
            (CallFunction|SetReady :!label _label_3))))
      (else
        (bind _currentitem_2 (Variables|/Game/Character/ThirdPersonBP/Blueprints/BP_Character.BP_Character_C|GetCurrentItem PlayerCharacter)
          (:then
            (if (Utilities|Enum|Equal(Enum) (Variables|/Game/Blueprints/Gameplay/Pickup_Items/ItemParent.ItemParent_C|GetItemName _currentitem_2) (Utilities|Text|FormatText "Empty Conical Flask"))
              (CallFunction|PlaceFlask _currentitem_2)
              (else
                (CallFunction|SetReady))))
          (:else
            (goto _label_3)))))))

(event EventLookat
  (params (PlayerCharacter :type BP%20Character%20Object%20Reference))
  ;[1 1 1] Update Look At Text for Solutions
  (bind _output_get (Variables|Default|SetPlayer PlayerCharacter))
  (if (== (Utilities|Array|LastIndex (Variables|Default|GetPlayersSolution)) 7)
    (Default|UpdateMessage (Variables|/Game/Character/ThirdPersonBP/Blueprints/BP_Character.BP_Character_C|GetPickupHUD (Variables|Default|GetPlayer)) "Solution Complete!")
    (else
      (bind _currentitem (Variables|/Game/Character/ThirdPersonBP/Blueprints/BP_Character.BP_Character_C|GetCurrentItem _output_get)
        (:then
          (if (Utilities|Enum|Equal(Enum) (Variables|/Game/Blueprints/Gameplay/Pickup_Items/ItemParent.ItemParent_C|GetItemName _currentitem) (Utilities|Text|FormatText "Empty Conical Flask"))
            ;[1 1 1] Update Message - Placing Conical Flask
            (if (Variables|Default|GetFlaskPlaced)
              (Default|UpdateMessage (Variables|/Game/Character/ThirdPersonBP/Blueprints/BP_Character.BP_Character_C|GetPickupHUD (Variables|Default|GetPlayer)) "Empty Conical Flask Already Placed")
              (else
                (Default|UpdateMessage (Variables|/Game/Character/ThirdPersonBP/Blueprints/BP_Character.BP_Character_C|GetPickupHUD (Variables|Default|GetPlayer)) "Place Empty Conical Flask")))
            (else
              (bind _array_element (Utilities|Array|ForEachLoopwithBreak (Variables|Default|GetNEW_Solution_List) :!label _label)
                (:LoopBody
                  (if (Utilities|Enum|Equal(Enum) (Utilities|Text|ToText(String) _array_element) (Variables|/Game/Blueprints/Gameplay/Pickup_Items/ItemParent.ItemParent_C|GetItemName _currentitem))
                    (Default|UpdateMessage (Variables|/Game/Character/ThirdPersonBP/Blueprints/BP_Character.BP_Character_C|GetPickupHUD (Variables|Default|GetPlayer)) (Utilities|Text|FormatText "Place {item}" (Variables|/Game/Blueprints/Gameplay/Pickup_Items/ItemParent.ItemParent_C|GetItemName _currentitem)))
                    (goto _label Break)
                    (else
                      (Default|UpdateMessage (Variables|/Game/Character/ThirdPersonBP/Blueprints/BP_Character.BP_Character_C|GetPickupHUD (Variables|Default|GetPlayer)) "Find a Solution to Add"))))))))
        (:else
          (CallFunction|HoldingNothing))))))

(event EventBeginPlay
  ;[1 1 1] Begin Play
  (bind _asstation_popup_wb (Utilities|Casting|CastToStationPopup_WB (UserInterface|GetUserWidgetObject (Variables|Default|GetPopup))))
  (Variables|Default|SetStationPopupREF _asstation_popup_wb)
  (CallFunction|SpawnSolutions)
  (bind _asbp_character (Utilities|Casting|CastToBP_Character (Game|GetPlayerCharacter 0)))
  (Variables|Default|SetCharacterREF _asbp_character)
  (Utilities|FlowControl|Sequence
    (:then_0
      ;[1 1 1] Random Solution
      (Utilities|Array|Shuffle (Variables|Default|GetNEW_Solution_Order)))))

(fn ConstructionScript
  (bind _returnvalue (Rendering|Material|CreateDynamicMaterialInstance (Variables|Default|GetBeaker) 1 0 "None" :!class /Script/Engine.PrimitiveComponent))
  (bind _output_get (Variables|Default|SetDynamicMaterial1 _returnvalue))
  (Rendering|Material|SetScalarParameterValue _output_get "Liquid_FillHeight" -0.5 :!class /Script/Engine.MaterialInstanceDynamic)
  (bind _returnvalue_2 (Rendering|Material|CreateDynamicMaterialInstance (Variables|Default|GetBeaker_Full) 1 0 "None" :!class /Script/Engine.PrimitiveComponent))
  (bind _output_get_2 (Variables|Default|SetDynamicMaterial2 _returnvalue_2))
  (Rendering|Material|SetScalarParameterValue _output_get_2 "Liquid_FillHeight" -0.5 :!class /Script/Engine.MaterialInstanceDynamic))