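; End-game trigger that returns the player to the main menu after the final microscope tutorial step.
; A repeating timer polls BP_MicroscopeNEW actors and enables sphere overlaps once one finishes; clearing its Looping flag never stops the timer.
; Player overlap plays the closing audio and, if Tutorial14Audio is valid, stops it, locks input and hides the cursor widget.
; That branch then shows a loading screen, fades out and opens MainMenu_Map.
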(event OnComponentBeginOverlap(Sphere)
  (params (OverlappedComponent :type Primitive%20Component%20Object%20Reference) (OtherActor :type Actor%20Object%20Reference) (OtherComp :type Primitive%20Component%20Object%20Reference) (OtherBodyIndex :type Integer) (bFromSweep :type Boolean) (SweepResult :type Hit%20Result%20Structure%20%28by%20ref%29))
  (bind _returnvalue (Game|GetPlayerController 0))
  (if (== OtherActor (Variables|Default|GetCharacterREF))
    (Utilities|FlowControl|Sequence
      (:then_0
        (bind _outactors (Actor|GetAllActorsOfClass "/Game/Blueprints/Gameplay/Interactive_Events/BP_MicroscopeNEW.BP_MicroscopeNEW_C"))
        (for _array_element _outactors
          (if (Variables|/Game/Blueprints/Gameplay/Interactive_Events/BP_MicroscopeNEW.BP_MicroscopeNEW_C|GetFinishedFinalTutorialStep _array_element)
            (Utilities|IsValid (Variables|/Game/Blueprints/Gameplay/Interactive_Events/BP_MicroscopeNEW.BP_MicroscopeNEW_C|GetTutorial_14Audio _array_element)
              (:Is%20Valid
                (Audio|Components|Audio|Stop (Variables|/Game/Blueprints/Gameplay/Interactive_Events/BP_MicroscopeNEW.BP_MicroscopeNEW_C|GetTutorial_14Audio _array_element))
                (Input|SetInputModeUIOnly _returnvalue 0 "DoNotLock")
                (Input|SetIgnoreMoveInput _returnvalue true)
                (Input|SetIgnoreLookInput _returnvalue true)
                (Widget|SetVisibility (Variables|/Game/UI/Objectives/NEWObjectivesHUD_WB.NEWObjectivesHUD_WB_C|GetRound_Mouse (Variables|/Game/Character/ThirdPersonBP/Blueprints/BP_Character.BP_Character_C|GetHUD_WB (Variables|Default|GetCharacterREF))) "Hidden")
                (Utilities|FlowControl|Delay 9.0)
                (Default|ShowEndGameLoadingScreen (Variables|Default|GetGameInstanceREF) 2 "Main Menu")
                (CameraFades|StartCameraFade :self (Game|GetPlayerCameraManager 0) :ToAlpha 1.0 :Duration 7.5 :bShouldFadeAudio true)
                (Utilities|FlowControl|Delay 7.5)
                (Game|OpenLevel(byName) "MainMenu_Map"))))))
      (:then_1
        (Utilities|FlowControl|Delay 0.5)
        (Audio|PlaySound2D "/Game/Audio/Tutorial_Voiceover/Tutorial_15.Tutorial_15" 1.0 1.0 0.0 0 0)))))

(event Custom|CheckForEndGame
  (bind _outactors (Actor|GetAllActorsOfClass "/Game/Blueprints/Gameplay/Interactive_Events/BP_MicroscopeNEW.BP_MicroscopeNEW_C"))
  (for _array_element _outactors
    (if (Variables|/Game/Blueprints/Gameplay/Interactive_Events/BP_MicroscopeNEW.BP_MicroscopeNEW_C|GetFinishedFinalTutorialStep _array_element)
      (Variables|/Script/Engine.PrimitiveComponent|SetbGenerateOverlapEvents (Variables|Default|GetSphere) true)
      (Variables|Default|SetLooping false))))

(event EventBeginPlay
  (Variables|/Script/Engine.PrimitiveComponent|SetbGenerateOverlapEvents (Variables|Default|GetSphere) false)
  (bind _asbp_character (Utilities|Casting|CastToBP_Character (Game|GetPlayerCharacter 0)))
  (Variables|Default|SetCharacterREF _asbp_character)
  (bind _asgame_info_instance (Utilities|Casting|CastToGameInfoInstance (Game|GetGameInstance)))
  (Variables|Default|SetGameInstanceREF _asgame_info_instance)
  (Utilities|Time|SetTimerbyEvent (delegate Custom|CheckForEndGame) 0.5 (Variables|Default|GetLooping)))

(fn ConstructionScript)