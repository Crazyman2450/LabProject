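; BP_LabDoorNEW is an interactive lab door that swings open automatically when the player character enters its trigger sphere.
; BeginPlay caches the player as BP_Character, and only that actor's overlap triggers the door.
; A DoorOpenClose timeline drives the yaw of SharedRoot, and after a fixed delay the same timeline reverses to close the door, whether or not the player has left the sphere.
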(event OnComponentBeginOverlap(Sphere)
  (params (OverlappedComponent :type Primitive%20Component%20Object%20Reference) (OtherActor :type Actor%20Object%20Reference) (OtherComp :type Primitive%20Component%20Object%20Reference) (OtherBodyIndex :type Integer) (bFromSweep :type Boolean) (SweepResult :type Hit%20Result%20Structure%20%28by%20ref%29))
  (if (== OtherActor (Variables|Character|GetCharacterREF))
    (CallFunction|DoorOpen)
    (Utilities|FlowControl|Delay 3.0)
    (CallFunction|DoorClose)))

(event Custom|DoorOpen
  (bind _rotation (Timeline|DoorOpenClose Play)
    (:Update
      (Transformation|SetRelativeRotation (Variables|Default|GetSharedRoot) (Math|Rotator|MakeRotator 0.0 0.0 (* _rotation -1e+02)) false false))))

(event Custom|DoorClose
  (bind _rotation (Timeline|DoorOpenClose Reverse)
    (:Update
      (Transformation|SetRelativeRotation (Variables|Default|GetSharedRoot) (Math|Rotator|MakeRotator 0.0 0.0 (* _rotation -1e+02)) false false))))

(event EventBeginPlay
  (bind _asbp_character (Utilities|Casting|CastToBP_Character (Game|GetPlayerCharacter 0)))
  (Variables|Character|SetCharacterREF _asbp_character))

(fn ConstructionScript)