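; Interactive brain slicer station that turns a held Brain Sample into a spawned Brain Slice item.
; Using it respawns the sample at its start transform, destroys the held one and locks the station until slicing finishes.
; Chained timelines, delays and sounds animate the arm and blade carriage, while a timer jitters the blade during the cut.
; Look-at updates HUD prompts by held item and state, and player overlap toggles the station popup.
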(event OnComponentBeginOverlap(OverlapCollision)
  (params (OverlappedComponent :type Primitive%20Component%20Object%20Reference) (OtherActor :type Actor%20Object%20Reference) (OtherComp :type Primitive%20Component%20Object%20Reference) (OtherBodyIndex :type Integer) (bFromSweep :type Boolean) (SweepResult :type Hit%20Result%20Structure%20%28by%20ref%29))
  (bind _station_popup_ref (Variables|Default|GetStation%20Popup%20REF))
  (if (== OtherActor (Variables|Default|GetCharacter%20REF))
    (Variables|/Game/UI/Gameplay/StationPopup_WB.StationPopup_WB_C|SetShowing _station_popup_ref true)
    (Variables|/Game/UI/Gameplay/StationPopup_WB.StationPopup_WB_C|SetTitle_Text _station_popup_ref "Brain Slicer")
    (Variables|Default|SetInRange? true)
    (Class|Image|SetBrush (Variables|/Game/UI/Gameplay/StationPopup_WB.StationPopup_WB_C|GetIcon_Image _station_popup_ref) (Utilities|Struct|MakeSlateBrush "(X=128.000000,Y=128.000000)" "(Left=0.000000,Top=0.000000,Right=0.000000,Bottom=0.000000)" "(SpecifiedColor=(R=1.000000,G=1.000000,B=1.000000,A=1.000000),ColorUseRule=UseColor_Specified)" "/Game/UI/UIAssets/Icon_Brain.Icon_Brain" "Image" "NoTile" "NoMirror"))
    (Variables|Default|SetInRange? true)))

(event OnComponentEndOverlap(OverlapCollision)
  (params (OverlappedComponent :type Primitive%20Component%20Object%20Reference) (OtherActor :type Actor%20Object%20Reference) (OtherComp :type Primitive%20Component%20Object%20Reference) (OtherBodyIndex :type Integer))
  (if (== OtherActor (Variables|Default|GetCharacter%20REF))
    (Variables|/Game/UI/Gameplay/StationPopup_WB.StationPopup_WB_C|SetShowing (Variables|Default|GetStation%20Popup%20REF) false)
    (Variables|Default|SetInRange? false)))

(event Custom|SliceEm
  (bind _brainslicer_bladearm (Variables|Default|GetBrainSlicer_BladeArm))
  (Rendering|SetVisibility (Variables|Default|GetBrain) true false)
  (bind _returnvalue (Audio|SpawnSoundatLocation "/Game/Audio/EquipmentSounds/ItemPickup.ItemPickup" (Transformation|GetWorldLocation (Variables|Default|GetPetri_Dish)) "0, 0, 0" 1.5 3.0 0.0 "/Game/Audio/EquipmentSounds/Fridge_Attentuation.Fridge_Attentuation" 0))
  (Audio|Components|Audio|Play _returnvalue 0.0)
  (Utilities|FlowControl|Delay 1.0)
  (bind _movetime (Timeline|Timeline_0 PlayFromStart)
    (:Update
      (Transformation|SetRelativeRotation (Variables|Default|GetArm_Rotate) (Math|Rotator|Lerp(Rotator) "0,45.000000, 0" "0, 0, 0" _movetime) false false))
    (:Finished
      (Utilities|FlowControl|Delay 2.0)
      (Utilities|FlowControl|Sequence
        (:then_0
          (bind _returnvalue_2 (Audio|SpawnSoundatLocation (Variables|Default|GetSound) (Transformation|GetWorldLocation _brainslicer_bladearm) "0, 0, 0" 1.0 1.0 0.0 "/Game/Audio/EquipmentSounds/Fridge_Attentuation.Fridge_Attentuation" 0))
          (Audio|Components|Audio|Play _returnvalue_2 0.2)
          (bind _movetime_2 (Timeline|Timeline_1 PlayFromStart)
            (:Update
              (Transformation|SetRelativeLocation _brainslicer_bladearm (Math|Vector|Lerp(Vector) "0, 0, 0" "0,6.000000, 0" _movetime_2) false false))
            (:Finished
              (Variables|Default|SetBladeLooping false)
              (Audio|Components|Audio|Stop _returnvalue_2)
              (Utilities|FlowControl|Sequence
                (:then_0
                  (Utilities|FlowControl|Delay 1.0)
                  (bind _time (Timeline|Timeline_2 Play)
                    (:Update
                      (Transformation|SetRelativeLocation (Variables|Default|GetBrainSlicer_BladeArm) (Math|Vector|Lerp(Vector) "0,6.000000, 0" "0, 0, 0" _time) false false))
                    (:Finished
                      (Audio|Components|Audio|Stop (stale _returnvalue_3))
                      (Utilities|FlowControl|Delay 0.5)
                      (bind _movetime_3 (Timeline|Timeline_3 PlayFromStart)
                        (:Update
                          (Transformation|SetRelativeRotation (Variables|Default|GetArm_Rotate) (Math|Rotator|Lerp(Rotator) "0, 0, 0" "0,45.000000, 0" _movetime_3) false false))
                        (:Finished
                          (Utilities|FlowControl|Sequence
                            (:then_0
                              ;[1 1 1] Pick up brain
                              (Utilities|FlowControl|Delay 1.0)
                              (Rendering|SetVisibility (Variables|Default|GetBrain) false false)
                              (Game|SpawnActorfromClass "/Game/Blueprints/Gameplay/Pickup_Items/BrainSlice.BrainSlice_C" (Transformation|GetWorldTransform (Variables|Default|GetSpawnPoint)) "Undefined" 0 "Brain Slice" "A slice of a brain specimen used to recored electrical activity in cells." 0.0 "(R=0.000000,G=0.000000,B=0.000000,A=0.000000)" 0)
                              (Default|UpdateMessage (Variables|/Game/Character/ThirdPersonBP/Blueprints/BP_Character.BP_Character_C|GetPickupHUD (Variables|Default|GetPlayer%20Character)) "Find a Brain Sample")
                              (Variables|Default|SetReady true))))))))
                (:then_1
                  (Utilities|FlowControl|Delay 0.75)
                  (bind _returnvalue_3 (Audio|SpawnSoundatLocation (Variables|Default|GetSound) (Transformation|GetWorldLocation (Variables|Default|GetBrainSlicer_BladeArm)) "0, 0, 0" 1.0 0.2 0.0 "/Game/Audio/EquipmentSounds/Fridge_Attentuation.Fridge_Attentuation" 0))
                  (Audio|Components|Audio|Play _returnvalue_3 1.0))))))
        (:then_1
          (Variables|Default|SetBladeLooping true)
          (Utilities|Time|SetTimerbyEvent (delegate Custom|Slicertron) 0.1 (Variables|Default|GetBladeLooping)))))))

(event Custom|Slicertron
  (if (Variables|Default|GetBladeLooping)
    (Transformation|SetRelativeLocation (Variables|Default|GetBrainSlicer_Blade) "-0.250000, 0, 0" false false)
    (Utilities|FlowControl|Delay 0.05)
    (Transformation|SetRelativeLocation (Variables|Default|GetBrainSlicer_Blade) "0.250000, 0, 0" false false)))

(event Custom|HoldingNothing
  ;[1 1 1] Holding Nothing
  (Default|UpdateMessage (Variables|/Game/Character/ThirdPersonBP/Blueprints/BP_Character.BP_Character_C|GetPickupHUD (Variables|Default|GetPlayer%20Character)) "Find a Brain Sample"))

(event EventBeginPlay
  (bind _asgame_info_instance (Utilities|Casting|CastToGameInfoInstance (Game|GetGameInstance)))
  (Variables|Default|SetGameInfoInstanceREF _asgame_info_instance)
  (bind _asbp_character (Utilities|Casting|CastToBP_Character (Game|GetPlayerCharacter 0)))
  (Variables|Default|SetCharacter%20REF _asbp_character)
  (bind _asstation_popup_wb (Utilities|Casting|CastToStationPopup_WB (UserInterface|GetUserWidgetObject (Variables|Default|GetPopup))))
  (bind _output_get (Variables|Default|SetStation%20Popup%20REF _asstation_popup_wb))
  (Variables|/Game/UI/Gameplay/StationPopup_WB.StationPopup_WB_C|SetInteractable _output_get false))

(event EventLookat
  (params (PlayerCharacter :type BP%20Character%20Object%20Reference))
  ;[1 1 1] Update Look At Text for Solutions
  (bind _output_get (Variables|Default|SetPlayer%20Character PlayerCharacter))
  (if (Variables|Default|GetReady)
    (bind _currentitem (Variables|/Game/Character/ThirdPersonBP/Blueprints/BP_Character.BP_Character_C|GetCurrentItem _output_get)
      (:then
        (if (Utilities|Enum|Equal(Enum) (Variables|/Game/Blueprints/Gameplay/Pickup_Items/ItemParent.ItemParent_C|GetItemName _currentitem) (Utilities|Text|FormatText "Brain Sample"))
          ;[1 1 1] Slice em up
          (Default|UpdateMessage (Variables|/Game/Character/ThirdPersonBP/Blueprints/BP_Character.BP_Character_C|GetPickupHUD (Variables|Default|GetPlayer%20Character)) "Slice Brain Sample")
          (else
            (Default|UpdateMessage (Variables|/Game/Character/ThirdPersonBP/Blueprints/BP_Character.BP_Character_C|GetPickupHUD (Variables|Default|GetPlayer%20Character)) "Find a Brain Sample"))))
      (:else
        (CallFunction|HoldingNothing)))
    (else
      (Default|UpdateMessage (Variables|/Game/Character/ThirdPersonBP/Blueprints/BP_Character.BP_Character_C|GetPickupHUD _output_get) "Brain Slicing in Progress"))))

(event EventUseItem
  (params (PlayerCharacter :type BP%20Character%20Object%20Reference))
  (if (Variables|Default|GetReady)
    (bind _currentitem (Variables|/Game/Character/ThirdPersonBP/Blueprints/BP_Character.BP_Character_C|GetCurrentItem PlayerCharacter)
      (:then
        (Variables|Default|SetReady false)
        (if (Utilities|Enum|Equal(Enum) (Variables|/Game/Blueprints/Gameplay/Pickup_Items/ItemParent.ItemParent_C|GetItemName _currentitem) (Utilities|Text|MakeLiteralText "Brain Sample"))
          (Game|SpawnActorfromClass "/Game/Blueprints/Gameplay/Pickup_Items/Brain.Brain_C" (Math|Transform|MakeTransform (.location (Variables|/Game/Blueprints/Gameplay/Pickup_Items/ItemParent.ItemParent_C|GetStart_Transform _currentitem)) (.rotation (Variables|/Game/Blueprints/Gameplay/Pickup_Items/ItemParent.ItemParent_C|GetStart_Transform _currentitem)) "1,1,1") "Undefined" 0 (Variables|/Game/Blueprints/Gameplay/Pickup_Items/ItemParent.ItemParent_C|GetItemName _currentitem) (Variables|/Game/Blueprints/Gameplay/Pickup_Items/ItemParent.ItemParent_C|GetItemDescription _currentitem) 0.0 "(R=0.000000,G=0.000000,B=0.000000,A=0.000000)" 0)
          (Actor|DestroyActor _currentitem)
          (Default|UpdateMessage (Variables|/Game/Character/ThirdPersonBP/Blueprints/BP_Character.BP_Character_C|GetPickupHUD (Variables|Default|GetPlayer%20Character)) "Brain Slicing in Progress")
          (CallFunction|SliceEm)
          (else
            (Variables|Default|SetReady true))))
      (:else))))

(fn ConstructionScript)