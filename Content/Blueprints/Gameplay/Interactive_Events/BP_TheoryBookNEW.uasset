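; Interactive book actor that opens theory content when the player interacts with it.
; Sphere overlap toggles the StationPopup widget and an in-range flag, while look-at updates the character's HUD prompt.
; Interact checks overlap, range, readiness and open state, then flashes the popup button, calls Theory01 on the game instance, switches to UI-only input with cursor and fades the camera.
; A separate SetReady event restores readiness after a debounce delay.
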(event OnComponentBeginOverlap(Sphere)
  (params (OverlappedComponent :type Primitive%20Component%20Object%20Reference) (OtherActor :type Actor%20Object%20Reference) (OtherComp :type Primitive%20Component%20Object%20Reference) (OtherBodyIndex :type Integer) (bFromSweep :type Boolean) (SweepResult :type Hit%20Result%20Structure%20%28by%20ref%29))
  (bind _stationpopupref (Variables|Default|GetStationPopupREF))
  ;[1 1 1] Show the description widget
  (if (== OtherActor (Variables|Default|GetCharacterREF))
    (Variables|/Game/UI/Gameplay/StationPopup_WB.StationPopup_WB_C|SetShowing _stationpopupref true)
    (Variables|/Game/UI/Gameplay/StationPopup_WB.StationPopup_WB_C|SetTitle_Text _stationpopupref "Theory Content")
    (Class|Image|SetBrush (Variables|/Game/UI/Gameplay/StationPopup_WB.StationPopup_WB_C|GetIcon_Image _stationpopupref) (Utilities|Struct|MakeSlateBrush "(X=128.000000,Y=128.000000)" "(Left=0.000000,Top=0.000000,Right=0.000000,Bottom=0.000000)" "(SpecifiedColor=(R=1.000000,G=1.000000,B=1.000000,A=1.000000),ColorUseRule=UseColor_Specified)" "/Game/UI/UIAssets/Clipboard_Icon.Clipboard_Icon" "Image" "NoTile" "NoMirror"))
    (Variables|Default|SetInRange? true)
    (Variables|/Game/UI/Gameplay/StationPopup_WB.StationPopup_WB_C|SetInteract_Term (Variables|Default|GetStationPopupREF) "Open")))

(event OnComponentEndOverlap(Sphere)
  (params (OverlappedComponent :type Primitive%20Component%20Object%20Reference) (OtherActor :type Actor%20Object%20Reference) (OtherComp :type Primitive%20Component%20Object%20Reference) (OtherBodyIndex :type Integer))
  ;[1 1 1] Show the description widget
  (if (== OtherActor (Variables|Default|GetCharacterREF))
    (Variables|/Game/UI/Gameplay/StationPopup_WB.StationPopup_WB_C|SetShowing (Variables|Default|GetStationPopupREF) false)
    (Variables|Default|SetInRange? false)))

(event Custom|SetReady
  ;[1 1 1] Set Ready
  (Utilities|FlowControl|Delay (Variables|Default|GetDebounceTime))
  (Variables|Default|SetReady true))

(event EventLookat
  (params (PlayerCharacter :type BP%20Character%20Object%20Reference))
  ;[1 1 1] Update Look At Text for Solutions
  (Default|UpdateMessage (Variables|/Game/Character/ThirdPersonBP/Blueprints/BP_Character.BP_Character_C|GetPickupHUD (Variables|Default|GetCharacterREF)) "Open Theory Content"))

(event EventInteract
  (params (PlayerInteracted :type Actor%20Object%20Reference))
  (bind _returnvalue (Game|GetPlayerController 0))
  (bind _stationpopupref (Variables|Default|GetStationPopupREF))
  (bind _isoverlapping_ (Default|CharacterOverlappingItem (Variables|Default|GetGameInstanceREF) PlayerInteracted (Variables|Default|GetSphere)))
  (if _isoverlapping_
    (if (Variables|Default|GetInRange?)
      (if (Variables|Default|GetReady)
        (if (not (Variables|Default|GetTheoryOpen))
          (Variables|Default|SetTheoryOpen true)
          (Variables|Default|SetReady false)
          (Variables|/Game/UI/Gameplay/StationPopup_WB.StationPopup_WB_C|SetButtonDown _stationpopupref true)
          (Utilities|FlowControl|Delay 0.1)
          (Variables|/Game/UI/Gameplay/StationPopup_WB.StationPopup_WB_C|SetButtonDown _stationpopupref false)
          (Default|Theory01 (Variables|Default|GetGameInstanceREF))
          (Input|SetInputModeUIOnly _returnvalue 0 "DoNotLock")
          (Variables|/Script/Engine.PlayerController|SetbShowMouseCursor _returnvalue true)
          (CameraFades|StartCameraFade :self (Game|GetPlayerCameraManager 0) :ToAlpha 1.0 :Duration 0.5 :bHoldWhenFinished true)
          (Utilities|FlowControl|Delay 1.0))))))

(event EventBeginPlay
  ;[1 1 1] Begin Play
  (bind _asstation_popup_wb (Utilities|Casting|CastToStationPopup_WB (UserInterface|GetUserWidgetObject (Variables|Default|GetPopup))))
  (Variables|Default|SetStationPopupREF _asstation_popup_wb)
  (bind _asbp_character (Utilities|Casting|CastToBP_Character (Game|GetPlayerCharacter 0)))
  (Variables|Default|SetCharacterREF _asbp_character)
  (bind _asgame_info_instance (Utilities|Casting|CastToGameInfoInstance (Game|GetGameInstance)))
  (Variables|Default|SetGameInstanceREF _asgame_info_instance))

(fn ConstructionScript)