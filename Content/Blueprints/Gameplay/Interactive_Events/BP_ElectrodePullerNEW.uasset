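; Interactive pipette puller station that turns a held Glass Pipette into a Microelectrode the player can collect.
; Look-at prompts and item use follow the Ready and ReadyToPickup flags, and an overlap volume toggles the station popup.
; Use respawns the pipette at its start transform, destroys the held one and runs PullEm, a chained Timeline animation of bars, lid and laser.
; An unconnected Brain Sample branch never runs.
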(event OnComponentBeginOverlap(OverlapCollision)
  (params (OverlappedComponent :type Primitive%20Component%20Object%20Reference) (OtherActor :type Actor%20Object%20Reference) (OtherComp :type Primitive%20Component%20Object%20Reference) (OtherBodyIndex :type Integer) (bFromSweep :type Boolean) (SweepResult :type Hit%20Result%20Structure%20%28by%20ref%29))
  (bind _station_popup_ref (Variables|Default|GetStation%20Popup%20REF))
  (if (== OtherActor (Variables|Default|GetCharacter%20REF))
    (Variables|/Game/UI/Gameplay/StationPopup_WB.StationPopup_WB_C|SetShowing _station_popup_ref true)
    (Variables|/Game/UI/Gameplay/StationPopup_WB.StationPopup_WB_C|SetTitle_Text _station_popup_ref "Pipette Puller")
    (Variables|Default|SetInRange? true)
    (Class|Image|SetBrush (Variables|/Game/UI/Gameplay/StationPopup_WB.StationPopup_WB_C|GetIcon_Image _station_popup_ref) (Utilities|Struct|MakeSlateBrush "(X=128.000000,Y=128.000000)" "(Left=0.000000,Top=0.000000,Right=0.000000,Bottom=0.000000)" "(SpecifiedColor=(R=1.000000,G=1.000000,B=1.000000,A=1.000000),ColorUseRule=UseColor_Specified)" "/Game/UI/UIAssets/Icon_Puller.Icon_Puller" "Image" "NoTile" "NoMirror"))
    (Variables|Default|SetInRange? true)))

(event OnComponentEndOverlap(OverlapCollision)
  (params (OverlappedComponent :type Primitive%20Component%20Object%20Reference) (OtherActor :type Actor%20Object%20Reference) (OtherComp :type Primitive%20Component%20Object%20Reference) (OtherBodyIndex :type Integer))
  (if (== OtherActor (Variables|Default|GetCharacter%20REF))
    (Variables|/Game/UI/Gameplay/StationPopup_WB.StationPopup_WB_C|SetShowing (Variables|Default|GetStation%20Popup%20REF) false)
    (Variables|Default|SetInRange? false)))

(event Custom|PullEm
  (Utilities|FlowControl|Delay 0.5)
  (Rendering|SetVisibility (Variables|Default|GetElectrodePuller_Pipette_Unpulled) true false)
  (Utilities|FlowControl|Delay 0.5)
  (bind _time (Timeline|Timeline_0 PlayFromStart)
    (:Update
      (Transformation|SetRelativeLocation (Variables|Default|GetElectrodePuller_Bar_Right) (Math|Vector|Lerp(Vector) "0, 0, 0" "-3.500000,0.000000, 0" _time) false false)
      (Transformation|SetRelativeLocation (Variables|Default|GetElectrodePuller_Bar_Left) (Math|Vector|Lerp(Vector) "0, 0, 0" "3.500000,0.000000, 0" _time) false false))
    (:Finished
      (Utilities|FlowControl|Delay 0.5)
      (Utilities|FlowControl|Sequence
        (:then_0
          (bind _time_2 (Timeline|Timeline_1 PlayFromStart)
            (:Update
              (Transformation|SetRelativeRotation (Variables|Default|GetLidScene) (Math|Rotator|Lerp(Rotator) "0, 0,-180.000000" "0, 0, 0" _time_2) false false))
            (:Finished
              (Utilities|FlowControl|Delay 0.5)
              (Rendering|SetVisibility (Variables|Default|GetLaser) true false)
              (Utilities|FlowControl|Delay 0.5)
              (bind _time_3 (Timeline|Timeline_2 PlayFromStart)
                (:Update
                  (Transformation|SetRelativeLocation (Variables|Default|GetElectrodePuller_Bar_Right) (Math|Vector|Lerp(Vector) "-3.500000,0.000000, 0" "-2.500000,0.000000, 0" _time_3) false false)
                  (Transformation|SetRelativeLocation (Variables|Default|GetElectrodePuller_Bar_Left) (Math|Vector|Lerp(Vector) "3.500000, 0, 0" "2.500000,0.000000, 0" _time_3) false false))
                (:Finished
                  (Rendering|SetVisibility (Variables|Default|GetElectrodePuller_Pipette_Right) true false)
                  (Rendering|SetVisibility (Variables|Default|GetLaser) false false)
                  (Utilities|FlowControl|Delay 1.0)
                  (Rendering|SetVisibility (Variables|Default|GetLaser) true false)
                  (Utilities|FlowControl|Delay 0.5)
                  (bind _time_4 (Timeline|Timeline_3 PlayFromStart)
                    (:Update
                      (Transformation|SetRelativeLocation (Variables|Default|GetElectrodePuller_Bar_Right) (Math|Vector|Lerp(Vector) "-2.500000,0.000000, 0" "0, 0, 0" _time_4) false false)
                      (Transformation|SetRelativeLocation (Variables|Default|GetElectrodePuller_Bar_Left) (Math|Vector|Lerp(Vector) "2.500000, 0, 0" "0, 0, 0" _time_4) false false))
                    (:Finished
                      (Utilities|FlowControl|Delay 0.5)
                      (Rendering|SetVisibility (Variables|Default|GetLaser) false false)
                      (Utilities|FlowControl|Delay 0.5)
                      (bind _time_5 (Timeline|Timeline_4 PlayFromStart)
                        (:Update
                          (Transformation|SetRelativeRotation (Variables|Default|GetLidScene) (Math|Rotator|Lerp(Rotator) "0, 0, 0" "0, 0,-180.000000" _time_5) false false)
                          (Default|UpdateMessage (Variables|/Game/Character/ThirdPersonBP/Blueprints/BP_Character.BP_Character_C|GetPickupHUD (Variables|Default|GetPlayer%20Character)) "Pick up Micropipette")
                          (Variables|Default|SetReadyToPickup true)
                          (Variables|Default|SetReady true))))))))))
        (:then_1
          (Utilities|FlowControl|Delay 0.8)
          (bind _returnvalue (Audio|SpawnSoundatLocation "/Game/Audio/EquipmentSounds/FridgeClosed.FridgeClosed" (Transformation|GetWorldLocation (Variables|Default|GetElectrodePuller_Body)) "0, 0, 0" 0.75 1e+01 0.0 0 0))
          (Audio|Components|Audio|Play _returnvalue 0.0))))))

(event Custom|HoldingNothing
  ;[1 1 1] Holding Nothing
  (Default|UpdateMessage (Variables|/Game/Character/ThirdPersonBP/Blueprints/BP_Character.BP_Character_C|GetPickupHUD (Variables|Default|GetPlayer%20Character)) "Find a Glass Pipette"))

(event EventBeginPlay
  (bind _asgame_info_instance (Utilities|Casting|CastToGameInfoInstance (Game|GetGameInstance)))
  (Variables|Default|SetGameInfoInstanceREF _asgame_info_instance)
  (bind _asbp_character (Utilities|Casting|CastToBP_Character (Game|GetPlayerCharacter 0)))
  (Variables|Default|SetCharacter%20REF _asbp_character)
  (bind _asstation_popup_wb (Utilities|Casting|CastToStationPopup_WB (UserInterface|GetUserWidgetObject (Variables|Default|GetPopup))))
  (bind _output_get (Variables|Default|SetStation%20Popup%20REF _asstation_popup_wb))
  (Variables|/Game/UI/Gameplay/StationPopup_WB.StationPopup_WB_C|SetInteractable _output_get false))

(event EventLookat
  (params (PlayerCharacter :type BP%20Character%20Object%20Reference))
  ;[1 1 1] Update Look At Text for Solutions
  (bind _output_get (Variables|Default|SetPlayer%20Character PlayerCharacter))
  (if (Variables|Default|GetReady)
    (if (Variables|Default|GetReadyToPickup)
      (Default|UpdateMessage (Variables|/Game/Character/ThirdPersonBP/Blueprints/BP_Character.BP_Character_C|GetPickupHUD _output_get) "Pick up Micropipette")
      (else
        (bind _currentitem (Variables|/Game/Character/ThirdPersonBP/Blueprints/BP_Character.BP_Character_C|GetCurrentItem _output_get)
          (:then
            (if (Utilities|Enum|Equal(Enum) (Variables|/Game/Blueprints/Gameplay/Pickup_Items/ItemParent.ItemParent_C|GetItemName _currentitem) (Utilities|Text|FormatText "Glass Pipette"))
              ;[1 1 1] Pull em up
              (Default|UpdateMessage (Variables|/Game/Character/ThirdPersonBP/Blueprints/BP_Character.BP_Character_C|GetPickupHUD (Variables|Default|GetPlayer%20Character)) "Pull Pipette")
              (else
                (Default|UpdateMessage (Variables|/Game/Character/ThirdPersonBP/Blueprints/BP_Character.BP_Character_C|GetPickupHUD (Variables|Default|GetPlayer%20Character)) "Find a Glass Pipette"))))
          (:else
            (CallFunction|HoldingNothing)))))
    (else
      (Default|UpdateMessage (Variables|/Game/Character/ThirdPersonBP/Blueprints/BP_Character.BP_Character_C|GetPickupHUD _output_get) "Pipette Pulling in Progress"))))

(event EventUseItem
  (params (PlayerCharacter :type BP%20Character%20Object%20Reference))
  (if (Variables|Default|GetReady)
    (if (Variables|Default|GetReadyToPickup)
      (Variables|/Game/Character/ThirdPersonBP/Blueprints/BP_Character.BP_Character_C|GetCurrentItem PlayerCharacter
        (:then)
        (:else
          (bind _returnvalue (Game|SpawnActorfromClass "/Game/Blueprints/Gameplay/Pickup_Items/Microelectrode.Microelectrode_C" (Math|Transform|MakeTransform "0,0.000000,5000.000000") "Undefined" 0 "Microelectrode" "The pulled electrode is used to stimulate individual cells electrically and to study electrical potentials in them." 0.0 "(R=0.000000,G=0.000000,B=0.000000,A=0.000000)" 0))
          (Default|PickUpItemPractical _returnvalue)
          (Default|UpdateMessage (Variables|/Game/Character/ThirdPersonBP/Blueprints/BP_Character.BP_Character_C|GetPickupHUD (Variables|Default|GetPlayer%20Character)) "Find a Glass Capillary Tube")
          (Variables|Default|SetReadyToPickup false)))
      (else
        (bind _currentitem (Variables|/Game/Character/ThirdPersonBP/Blueprints/BP_Character.BP_Character_C|GetCurrentItem PlayerCharacter)
          (:then
            (Variables|Default|SetReady false)
            (if (Utilities|Enum|Equal(Enum) (Variables|/Game/Blueprints/Gameplay/Pickup_Items/ItemParent.ItemParent_C|GetItemName _currentitem) (Utilities|Text|MakeLiteralText "Glass Pipette"))
              (Game|SpawnActorfromClass "/Game/Blueprints/Gameplay/Pickup_Items/GlassPipette.GlassPipette_C" (Math|Transform|MakeTransform (.location (Variables|/Game/Blueprints/Gameplay/Pickup_Items/ItemParent.ItemParent_C|GetStart_Transform _currentitem)) (.rotation (Variables|/Game/Blueprints/Gameplay/Pickup_Items/ItemParent.ItemParent_C|GetStart_Transform _currentitem)) "1,1,1") "Undefined" 0 (Variables|/Game/Blueprints/Gameplay/Pickup_Items/ItemParent.ItemParent_C|GetItemName _currentitem) (Variables|/Game/Blueprints/Gameplay/Pickup_Items/ItemParent.ItemParent_C|GetItemDescription _currentitem) 0.0 "(R=0.000000,G=0.000000,B=0.000000,A=0.000000)" 0)
              (Actor|DestroyActor _currentitem)
              (Default|UpdateMessage (Variables|/Game/Character/ThirdPersonBP/Blueprints/BP_Character.BP_Character_C|GetPickupHUD (Variables|Default|GetPlayer%20Character)) "Pipette Pulling in Progress")
              (CallFunction|PullEm)
              (else
                (Variables|Default|SetReady true))))
          (:else))))))

(fn ConstructionScript)