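; Interactive glass cabinet with two doors that swing open and shut when the player interacts within range.
; An overlap box drives a station popup with Open/Close prompts; Interact checks range and a Ready lock before toggling.
; Paired timelines rotate the doors forward or in reverse with sound; DoorOpen is inverted, true while shut.
; In Tutorial_Map, the first opening also fades the HUD's pickup controls.
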(event OnComponentBeginOverlap(OverlapCollision)
  (params (OverlappedComponent :type Primitive%20Component%20Object%20Reference) (OtherActor :type Actor%20Object%20Reference) (OtherComp :type Primitive%20Component%20Object%20Reference) (OtherBodyIndex :type Integer) (bFromSweep :type Boolean) (SweepResult :type Hit%20Result%20Structure%20%28by%20ref%29))
  (bind _stationpopupref (Variables|Default|GetStationPopupREF))
  (bind _stationpopupref_2 (Variables|Default|GetStationPopupREF))
  (if (== OtherActor (Variables|Default|GetCharacterREF))
    (Variables|/Game/UI/Gameplay/StationPopup_WB.StationPopup_WB_C|SetShowing _stationpopupref_2 true)
    (Variables|/Game/UI/Gameplay/StationPopup_WB.StationPopup_WB_C|SetTitle_Text _stationpopupref_2 "Cabinet")
    (Variables|Default|SetInRange? true)
    (Class|Image|SetBrush (Variables|/Game/UI/Gameplay/StationPopup_WB.StationPopup_WB_C|GetIcon_Image _stationpopupref_2) (Utilities|Struct|MakeSlateBrush "(X=128.000000,Y=128.000000)" "(Left=0.000000,Top=0.000000,Right=0.000000,Bottom=0.000000)" "(SpecifiedColor=(R=1.000000,G=1.000000,B=1.000000,A=1.000000),ColorUseRule=UseColor_Specified)" "/Game/UI/UIAssets/Icon_Cabinet.Icon_Cabinet" "Image" "NoTile" "NoMirror"))
    (Variables|Default|SetInRange? true)
    (if (Variables|Default|GetDoorOpen)
      (Variables|/Game/UI/Gameplay/StationPopup_WB.StationPopup_WB_C|SetInteract_Term _stationpopupref "Open")
      (else
        (Variables|/Game/UI/Gameplay/StationPopup_WB.StationPopup_WB_C|SetInteract_Term _stationpopupref "Close")))))

(event OnComponentEndOverlap(OverlapCollision)
  (params (OverlappedComponent :type Primitive%20Component%20Object%20Reference) (OtherActor :type Actor%20Object%20Reference) (OtherComp :type Primitive%20Component%20Object%20Reference) (OtherBodyIndex :type Integer))
  (if (== OtherActor (Variables|Default|GetCharacterREF))
    (Variables|/Game/UI/Gameplay/StationPopup_WB.StationPopup_WB_C|SetShowing (Variables|Default|GetStationPopupREF) false)
    (Variables|Default|SetInRange? false)))

(event Custom|ToggleDoors
  (params (Direction :type Boolean))
  (bind _stationpopupref (Variables|Default|GetStationPopupREF))
  (bind _popup (Variables|Default|GetPopup))
  (bind _returnvalue (Transformation|GetWorldLocation _popup))
  (if (Variables|Default|GetDoorOpen)
    (Variables|Default|SetDoorOpen false)
    (Variables|/Game/UI/Gameplay/StationPopup_WB.StationPopup_WB_C|SetInteract_Term _stationpopupref "Close")
    (Utilities|FlowControl|Sequence
      (:then_0
        (bind _doortimeopenright (Timeline|Timeline_0 PlayFromStart)
          (:Update
            (Transformation|SetRelativeRotation (Variables|Default|GetDoorOpenRight) (Math|Rotator|MakeRotator 0.0 0.0 (* _doortimeopenright (Variables|Default|GetDoorAngleRight))) false false))
          (:Finished
            (Variables|Default|SetReady true :!label _label))))
      (:then_1
        (bind _doortimeopenleft (Timeline|Timeline_1 PlayFromStart)
          (:Update
            (Transformation|SetRelativeRotation (Variables|Default|GetDoorOpenLeft) (Math|Rotator|MakeRotator 0.0 0.0 (* _doortimeopenleft (Variables|Default|GetDoorAngleLeft))) false false))
          (:Finished
            (goto _label))))
      (:then_2
        (Utilities|FlowControl|Delay 0.0)
        (Audio|PlaySoundatLocation "/Game/Audio/Door_Open_3.Door_Open_3" _returnvalue "0, 0, 0" 0.5 3.0 0.15 0 0 0)))
    (else
      (Variables|Default|SetDoorOpen true)
      (Variables|/Game/UI/Gameplay/StationPopup_WB.StationPopup_WB_C|SetInteract_Term _stationpopupref "Open")
      (Utilities|FlowControl|Sequence
        (:then_0
          (Timeline|Timeline_0 ReverseFromEnd))
        (:then_1
          (Timeline|Timeline_1 ReverseFromEnd))
        (:then_2
          (Utilities|FlowControl|Delay 0.3)
          (Audio|PlaySoundatLocation "/Game/Audio/Door_Close_1.Door_Close_1" _returnvalue "0, 0, 0" 0.3 1.0 0.0 0 0 0))))))

(event EventBeginPlay
  (|CallParentFunction)
  (bind _asgame_info_instance (Utilities|Casting|CastToGameInfoInstance (Game|GetGameInstance)))
  (Variables|Default|SetGameInfoInstance _asgame_info_instance)
  (bind _asbp_character (Utilities|Casting|CastToBP_Character (Game|GetPlayerCharacter 0)))
  (Variables|Default|SetCharacterREF _asbp_character)
  (bind _asstation_popup_wb (Utilities|Casting|CastToStationPopup_WB (UserInterface|GetUserWidgetObject (Variables|Default|GetPopup))))
  (Variables|Default|SetStationPopupREF _asstation_popup_wb))

(event EventInteract
  (params (PlayerInteracted :type Actor%20Object%20Reference))
  (bind _stationpopupref (Variables|Default|GetStationPopupREF))
  (bind _isoverlapping_ (Default|CharacterOverlappingItem (Variables|Default|GetGameInfoInstance) PlayerInteracted (Variables|Default|GetOverlapCollision)))
  (if _isoverlapping_
    (if (Variables|Default|GetInRange?)
      (if (Variables|Default|GetReady)
        (Variables|Default|SetReady false)
        (Variables|/Game/UI/Gameplay/StationPopup_WB.StationPopup_WB_C|SetButtonDown _stationpopupref true)
        (Utilities|FlowControl|Delay 0.1)
        (Variables|/Game/UI/Gameplay/StationPopup_WB.StationPopup_WB_C|SetButtonDown _stationpopupref false)
        (if (Variables|Default|GetDoorOpen)
          (CallFunction|ToggleDoors false)
          (bind _returnvalue (Game|GetCurrentLevelName true))
          (if (Utilities|Enum|Equal(Enum) _returnvalue "Tutorial_Map")
            (Utilities|FlowControl|Delay 0.5)
            (Utilities|FlowControl|DoOnce false
              (:Completed
                (Default|FadePickupControls (Variables|/Game/Character/ThirdPersonBP/Blueprints/BP_Character.BP_Character_C|GetHUD_WB (Variables|Default|GetCharacterREF))))))
          (else
            (CallFunction|ToggleDoors true)))))))

(fn ConstructionScript)