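; BP_MicroscopeControls is a trigger actor for the microscope controls step of what appears to be a tutorial.
; Its Sphere starts with overlap events off, and nothing in this Blueprint turns them on.
; When the player character overlaps it, it calls FadeMicroscopeControls on the HUD and disables itself.
; It then enables overlap on every BP_MicroscopeNEW sphere and stops Tutorial07Audio on every BP_PreparationAreaNEW.
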(event OnComponentBeginOverlap(Sphere)
  (params (OverlappedComponent :type Primitive%20Component%20Object%20Reference) (OtherActor :type Actor%20Object%20Reference) (OtherComp :type Primitive%20Component%20Object%20Reference) (OtherBodyIndex :type Integer) (bFromSweep :type Boolean) (SweepResult :type Hit%20Result%20Structure%20%28by%20ref%29))
  (if (== OtherActor (Variables|Default|GetCharacterREF))
    (Utilities|FlowControl|Sequence
      (:then_0
        (Default|FadeMicroscopeControls (Variables|/Game/Character/ThirdPersonBP/Blueprints/BP_Character.BP_Character_C|GetHUD_WB (Variables|Default|GetCharacterREF)))
        (Variables|/Script/Engine.PrimitiveComponent|SetbGenerateOverlapEvents (Variables|Default|GetSphere) false)
        (bind _outactors (Actor|GetAllActorsOfClass "/Game/Blueprints/Gameplay/Interactive_Events/BP_MicroscopeNEW.BP_MicroscopeNEW_C"))
        (for _array_element _outactors
          (Variables|/Script/Engine.PrimitiveComponent|SetbGenerateOverlapEvents (Variables|/Game/Blueprints/Gameplay/Interactive_Events/BP_MicroscopeNEW.BP_MicroscopeNEW_C|GetSphere _array_element) true)))
      (:then_1
        (bind _outactors_2 (Actor|GetAllActorsOfClass "/Game/Blueprints/Gameplay/Interactive_Events/BP_PreparationAreaNEW.BP_PreparationAreaNEW_C"))
        (for _array_element_2 _outactors_2
          (Utilities|IsValid (Variables|/Game/Blueprints/Gameplay/Interactive_Events/BP_PreparationAreaNEW.BP_PreparationAreaNEW_C|GetTutorial_07Audio _array_element_2)
            (:Is%20Valid
              (Audio|Components|Audio|Stop (Variables|/Game/Blueprints/Gameplay/Interactive_Events/BP_PreparationAreaNEW.BP_PreparationAreaNEW_C|GetTutorial_07Audio _array_element_2)))))))))

(event EventBeginPlay
  (Variables|/Script/Engine.PrimitiveComponent|SetbGenerateOverlapEvents (Variables|Default|GetSphere) false)
  (bind _asbp_character (Utilities|Casting|CastToBP_Character (Game|GetPlayerCharacter 0)))
  (Variables|Default|SetCharacterREF _asbp_character))

(fn ConstructionScript)