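; Blueprint helper that switches an outline on or off for a given actor through the custom depth stencil.
; Set Outline walks all descendants of the actor's root component, leaving out the root itself, and casts each to a primitive component.
; It toggles custom depth rendering on those primitives, writing a fixed stencil value when shown and clearing it when hidden.
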(fn SetOutline
  (params (Actor :type Actor%20Object%20Reference) (ShowOutline :type Boolean))
  (bind _rootcomponent (Variables|/Script/Engine.Actor|GetRootComponent Actor))
  (Utilities|IsValid _rootcomponent
    (:Is%20Valid
      (for _array_element (Components|GetChildrenComponents _rootcomponent true)
        (Utilities|IsValid _array_element
          (:Is%20Valid
            (bind _asprimitive_component (Utilities|Casting|CastToPrimitiveComponent _array_element))
            (if ShowOutline
              (Rendering|SetRenderCustomDepth _asprimitive_component true)
              (Rendering|SetCustomDepthStencilValue _asprimitive_component 2)
              (else
                (Rendering|SetRenderCustomDepth _asprimitive_component false)
                (Rendering|SetCustomDepthStencilValue _asprimitive_component 0)))))))))